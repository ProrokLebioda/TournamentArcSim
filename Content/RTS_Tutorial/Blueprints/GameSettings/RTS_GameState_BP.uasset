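; Game state for an RTS that runs the in-game clock and calendar at an adjustable speed.
; BeginPlay caches the player controller and seeds time, date and default speed.
; Each tick advances time through SetGameTime, splits it into clock units, rolls days into months and years, and pushes both to the controller's HUD widget.
; UpdateGameSpeed scales the default speed and calls CallGameSpeedController; SetGameClock and SetGameCalendar are stubs returning false.
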(event EventBeginPlay
  (Utilities|FlowControl|Sequence
    (:then_0
      (Utilities|ReferenceCasts))
    (:then_1
      ;[1 1 1] Set Default Game Clock & Calendar
      (Variables|GameSpeedSettings|SetGameTime (+ (Math|Conversions|ToFloat(Integer) (Variables|Clock|GetHours)) (/ (Math|Conversions|ToFloat(Integer) (Variables|Clock|GetMinutes)) 6e+01) (/ (Math|Conversions|ToFloat(Integer) (Variables|Clock|GetHours)) 3.6e+03)))
      (Variables|Calendar|SetGameDate (Utilities|Array|MakeArray (Variables|Calendar|GetDay) (Variables|Calendar|GetMonth) (Variables|Calendar|GetYear))))
    (:then_2
      ;[1 1 1] Set Default Game Speed
      (Variables|GameSpeedSettings|SetGameSpeed (Variables|GameSpeedSettings|GetDefaultGameSpeed)))))

(event EventTick
  (params (DeltaSeconds :type Float%20%28single-precision%29))
  ;[1 1 1] Update Game Clock & Calendar
  (Variables|GameSpeedSettings|SetGameTime (.GameTime (CallFunction|SetGameTime DeltaSeconds (Variables|GameSpeedSettings|GetGameSpeed) (Variables|GameSpeedSettings|GetGameTime))))
  (Variables|Calendar|SetDayCounter (.DayCount (CallFunction|SetGameTime DeltaSeconds (Variables|GameSpeedSettings|GetGameSpeed) (Variables|GameSpeedSettings|GetGameTime))))
  (CallFunction|SetClock)
  (CallFunction|SetCalendar))

(event EventUpdateGameSpeed
  (params (SpeedMultiplier :type Float%20%28single-precision%29))
  ;[1 1 1] Update Game Speed
  (bind _output_get (Variables|GameSpeedSettings|SetSpeedMultiplier SpeedMultiplier))
  (bind _output_get_2 (Variables|GameSpeedSettings|SetGameSpeed (* _output_get (Variables|GameSpeedSettings|GetDefaultGameSpeed))))
  (Default|CallGameSpeedController _output_get_2))

(fn ConstructionScript)

(fn SetClock
  (bind _gametime (Variables|GameSpeedSettings|GetGameTime))
  (bind _returnvalue (* _gametime 3.6e+03))
  (bind (_remainder _returnvalue_2) (Math|Float|Division(WholeandRemainder) _returnvalue 6e+01))
  (bind _returnvalue_3 (Math|Conversions|ToFloat(Integer) _returnvalue_2))
  (bind (_remainder_2 _returnvalue_4) (Math|Float|Division(WholeandRemainder) _returnvalue_3 6e+01))
  (Variables|Clock|SetSeconds (Math|Float|Floor _remainder))
  (Variables|Clock|SetMinutes (Math|Float|Floor _remainder_2))
  (Variables|Clock|SetHours (Math|Float|Floor (.Remainder (Math|Float|Division(WholeandRemainder) (Math|Conversions|ToFloat(Integer) _returnvalue_4) 24.0))))
  (bind _output_get (Variables|Calendar|SetGameDate (Utilities|Array|MakeArray (Variables|Clock|GetSeconds) (Variables|Clock|GetMinutes) (Variables|Clock|GetHours))))
  (Class|RTSGameTimeIF|SetGameClock(Message) (Variables|/Game/RTS_Tutorial/Blueprints/Player/RTS_PlayerController_BP.RTS_PlayerController_BP_C|GetHUD_GameTimeRef (Variables|Default|GetConterollerRef)) _output_get))

(fn SetCalendar
  (bind _output_get (Variables|Calendar|SetDay (+ (Variables|Calendar|GetDay) (Variables|Calendar|GetDayCounter))))
  (if (> _output_get (Class|KismetMathLibrary|DaysinMonth (Variables|Calendar|GetYear) (Variables|Calendar|GetMonth)))
    (Variables|Calendar|SetDay 1)
    (Variables|Calendar|SetMonth (+ (Variables|Calendar|GetMonth) 1)))
  (if (> (Variables|Calendar|GetMonth) 12)
    (Variables|Calendar|SetMonth 1)
    (Variables|Calendar|SetYear (+ (Variables|Calendar|GetYear) 1)))
  (bind _output_get_2 (Variables|Calendar|SetGameDate (Utilities|Array|MakeArray (Variables|Calendar|GetDay) (Variables|Calendar|GetMonth) (Variables|Calendar|GetYear))))
  (Class|RTSGameTimeIF|SetGameCalendar(Message) (Variables|/Game/RTS_Tutorial/Blueprints/Player/RTS_PlayerController_BP.RTS_PlayerController_BP_C|GetHUD_GameTimeRef (Variables|Default|GetConterollerRef)) _output_get_2))

(fn GetGameSpeed
  (return (Variables|GameSpeedSettings|GetGameSpeed)))

(fn SetGameCalendar
  (params (GameDate :type Array%20of%20Integers))
  (return false))

(fn SetGameClock
  (params (GameTime :type Array%20of%20Integers))
  (return false))