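; RTS spawn volume that scatters resource actors over the landscape within its bounds, optionally at begin play and on a repeating timer.
; SpawnResource box-traces from random offsets in the bounds and spawns only where the hit is Landscape.
; Timed spawning starts only alongside begin-play spawning, skips while paused, and stops spawning once the requested total reaches the maximum.
; Tick recalculates the respawn time from game speed or custom settings, but the running timer keeps its initial interval.
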(event Custom|SpawnResourceOnTimer
  (if (not (Variables|/Game/RTS_Tutorial/Blueprints/Widgets/GameTime_HUD.GameTime_HUD_C|GetIsPaused (Variables|/Game/RTS_Tutorial/Blueprints/Player/RTS_PlayerController_BP.RTS_PlayerController_BP_C|GetHUD_GameTimeRef (Variables|References|GetPlayerControllerRef))))
    (if (and (Variables|Bool|GetIsSpawnedOnTimer) (< (Variables|ResourceSettings|GetTotalNumberSpawned) (Variables|ResourceSettings|GetMaxResourcesSpawned)))
      (CallFunction|SpawnResource (Variables|References|GetResourceRef) (Variables|ResourceSettings|GetNumOfResourcesSpawn))
      (Variables|ResourceSettings|SetTotalNumberSpawned (+ (Variables|ResourceSettings|GetNumOfResourcesSpawn) (Variables|ResourceSettings|GetTotalNumberSpawned))))))

(event Custom|GetGameSpeed
  (params (GameSpeed :type Float%20%28single-precision%29))
  (Variables|ResourceSettings|SetGameSpeed GameSpeed))

(event EventBeginPlay
  (Utilities|FlowControl|Sequence
    (:then_0
      (Utilities|ReferenceCasts))
    (:then_1
      (EventDispatchers|BindEventtoGameSpeedController (Variables|References|GetGameStateRef) (EventDispatchers|CreateEvent :!event Custom|GetGameSpeed))
      (bind _gamespeed (Default|GetGameSpeed (Variables|References|GetGameStateRef)))
      (Variables|ResourceSettings|SetGameSpeed _gamespeed)
      (CallFunction|SetResprawnTimer))
    (:then_2
      (if (Variables|Bool|GetIsSpawnOnBeginPlay)
        (CallFunction|SpawnResource (Variables|References|GetResourceRef) (Variables|ResourceSettings|GetNumOfResourcesSpawn))
        (Variables|ResourceSettings|SetTotalNumberSpawned (+ (Variables|ResourceSettings|GetNumOfResourcesSpawn) (Variables|ResourceSettings|GetTotalNumberSpawned)))
        (if (and (Variables|Bool|GetIsSpawnedOnTimer) (< (Variables|ResourceSettings|GetTotalNumberSpawned) (Variables|ResourceSettings|GetMaxResourcesSpawned)))
          (Utilities|Time|SetTimerbyEvent (EventDispatchers|CreateEvent :!event Custom|SpawnResourceOnTimer) (Variables|ResourceSettings|GetRespawnTime) true))))))

(event EventTick
  (params (DeltaSeconds :type Float%20%28single-precision%29))
  (CallFunction|SetResprawnTimer))

(fn ConstructionScript)

(fn SpawnResource
  (params (Resource :type RTS%20Resource%20Master%20BP%20Class%20Reference) (SpawnAmount :type Integer))
  (bind (_origin _boxextent) (Collision|GetActorBounds false false))
  (bind _z (Math|Vector|BreakVector _origin))
  (bind (_x _y) (Math|Vector|BreakVector _boxextent))
  (bind _returnvalue (* _y 2.0))
  (bind _returnvalue_2 (* _x 2.0))
  (bind _returnvalue_3 (- _y _returnvalue))
  (bind _returnvalue_4 (- _x _returnvalue_2))
  (bind _returnvalue_5 (Math|Random|RandomFloatinRange _returnvalue_3 _y))
  (bind _returnvalue_6 (Math|Random|RandomFloatinRange _returnvalue_4 _x))
  (bind _returnvalue_7 (Math|Vector|MakeVector _returnvalue_6 _returnvalue_5 _z))
  (bind _returnvalue_8 (+ _origin _returnvalue_7))
  (LocalVariables|SetResourceRefLocal Resource)
  (LocalVariables|SetSpawnAmountLocal SpawnAmount)
  (for _index (range 0 (LocalVariables|GetSpawnAmountLocal))
    (bind _outhit (Collision|BoxTraceByChannel (+ _returnvalue_8 "0, 0,200.000000") "0, 0, 0" (- _returnvalue_8 (Math|Vector|MakeVector 0.0 0.0 2e+02)) "0, 0, 0" "TraceTypeQuery1" false 0 "None"))
    (if (== (Utilities|GetClass (.HitActor (Collision|BreakHitResult _outhit))) "/Script/Landscape.Landscape")
      (Game|SpawnActorfromClass (LocalVariables|GetResourceRefLocal) (Math|Conversions|ToTransform(Vector) (.Location (Collision|BreakHitResult _outhit))) "Undefined" 0 0))))

(fn SetResprawnTimer
  (switch Utilities|FlowControl|Switch|SwitchonRespawnTimerEnum (Variables|References|GetTimeSetting)
    (:NewEnumerator1
      (Variables|ResourceSettings|SetRespawnTime 0.0))
    (:NewEnumerator2
      (Variables|ResourceSettings|SetRespawnTime (Variables|ResourceSettings|GetGameSpeed)))
    (:NewEnumerator3
      (Variables|ResourceSettings|SetRespawnTime (Variables|ResourceSettings|GetUserRespawnTimer)))
    (:NewEnumerator4
      (Variables|ResourceSettings|SetRespawnTime (* (Variables|ResourceSettings|GetUserRespawnTimer) (Variables|ResourceSettings|GetGameSpeed)))))
  (return (Variables|ResourceSettings|GetRespawnTime)))